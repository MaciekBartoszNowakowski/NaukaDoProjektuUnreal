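; Player character for the blue character, moved with top-down Enhanced Input controls.
; On BeginPlay it adds the IMC_TopDown mapping context for its player controller.
; IA_Move drives movement along fixed world axes scaled by PlayerSpeed, with X input taking priority over Y so there are no diagonals.
; It also records the active axis in Directionality and tracks whether move input is held in IsHoldingMove.
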(event Input|EnhancedActionEvents|EnhancedInputActionIA_Move
  (params (ActionValue :type Vector%202D%20Structure) (ElapsedSeconds :type Float%20%28double-precision%29) (TriggeredSeconds :type Float%20%28double-precision%29) (InputAction :type Input%20Action%20Object%20Reference :default "/Game/Character/Input/IA_Move.IA_Move"))
  (:Triggered
    (if (!= (.x ActionValue) 0.0)
      (Pawn|Input|AddMovementInput "1.000000,0.000000,0.000000" (* (.x ActionValue) (Variables|Default|GetPlayerSpeed)) false)
      (Variables|Default|SetDirectionality (Math|Vector2D|MakeVector2D (.x ActionValue) 0.0))
      (else
        (Pawn|Input|AddMovementInput "0.000000,-1.000000,0.000000" (* (.y ActionValue) (Variables|Default|GetPlayerSpeed)) false)
        (Variables|Default|SetDirectionality (Math|Vector2D|MakeVector2D 0.0 (.y ActionValue))))))
  (:Started
    (Variables|Default|SetIsHoldingMove true))
  (:Completed
    (Variables|Default|SetIsHoldingMove false)))

(event EventBeginPlay
  (bind _asplayer_controller (Utilities|Casting|CastToPlayerController (Pawn|GetController)))
  (Input|AddMappingContext (PlayerController|LocalPlayerSubsystems|GetEnhancedInputLocalPlayerSubsystem _asplayer_controller) "/Game/Character/Input/IMC_TopDown.IMC_TopDown" 0 "(bIgnoreAllPressedKeysUntilRelease=True,bForceImmediately=False,bNotifyUserSettings=False)"))

(fn ConstructionScript)