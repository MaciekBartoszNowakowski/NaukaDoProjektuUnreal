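; BP_SheepGate is a puzzle gate that opens when four sheep are inside its plane collision.
; Overlap begin and end events for BP_Sheep raise and lower a counter, which is printed on each entry.
; At four, after a short delay, a timeline rolls the gate anchor open.
; The timeline's update also gives the player's BP_TopDown_Char the prize item once, guarded by a PrizeGiven flag.
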(event OnComponentBeginOverlap(PlaneCollision)
  (params (OverlappedComponent :type Primitive%20Component%20Object%20Reference) (OtherActor :type Actor%20Object%20Reference) (OtherComp :type Primitive%20Component%20Object%20Reference) (OtherBodyIndex :type Integer) (bFromSweep :type Boolean) (SweepResult :type Hit%20Result%20Structure%20%28by%20ref%29))
  (Utilities|Casting|CastToBP_Sheep OtherActor)
  (Variables|Default|Setsheep_counter (+ 1 (Variables|Default|Getsheep_counter)))
  (Development|PrintString (Utilities|String|ToString(Integer) (Variables|Default|Getsheep_counter)))
  (if (== (Variables|Default|Getsheep_counter) 4)
    (Utilities|FlowControl|Delay 0.1)
    (bind _newtrack_0 (Timeline|DoorRotateTimeline PlayFromStart)
      (:Update
        (Transformation|SetRelativeRotation (Variables|Default|GetGateAncor) (Math|Rotator|MakeRotator _newtrack_0 0.0 0.0) false false)
        (bind _asbp_top_down_char (Utilities|Casting|CastToBP_TopDown_Char (Game|GetPlayerCharacter 0)))
        (if (not (Variables|Default|GetPrizeGiven))
          (Default|PickUpItemEvent _asbp_top_down_char (Variables|Default|GetPrize))
          (Variables|Default|SetPrizeGiven true))))))

(event OnComponentEndOverlap(PlaneCollision)
  (params (OverlappedComponent :type Primitive%20Component%20Object%20Reference) (OtherActor :type Actor%20Object%20Reference) (OtherComp :type Primitive%20Component%20Object%20Reference) (OtherBodyIndex :type Integer))
  (Utilities|Casting|CastToBP_Sheep OtherActor)
  (Variables|Default|Setsheep_counter (+ -1 (Variables|Default|Getsheep_counter))))

(event EventBeginPlay)

(event EventTick
  (params (DeltaSeconds :type Float%20%28single-precision%29)))

(fn ConstructionScript)