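; BP_Door is an interactable door that teleports the player character to the location stored in its NewLocation variable.
; Box overlap shows or hides the InteractionComunication component for any actor, then enables or disables player 0's input on the door only for BP_TopDown_Char.
; While input is enabled, pressing E prints a debug message and moves player character 0 there without sweeping.
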(event OnComponentBeginOverlap(Box)
  (params (OverlappedComponent :type Primitive%20Component%20Object%20Reference) (OtherActor :type Actor%20Object%20Reference) (OtherComp :type Primitive%20Component%20Object%20Reference) (OtherBodyIndex :type Integer) (bFromSweep :type Boolean) (SweepResult :type Hit%20Result%20Structure%20%28by%20ref%29))
  (Rendering|SetVisibility (Variables|Default|GetInteractionComunication) true false)
  (Utilities|Casting|CastToBP_TopDown_Char OtherActor)
  (Input|EnableInput (Game|GetPlayerController 0)))

(event OnComponentEndOverlap(Box)
  (params (OverlappedComponent :type Primitive%20Component%20Object%20Reference) (OtherActor :type Actor%20Object%20Reference) (OtherComp :type Primitive%20Component%20Object%20Reference) (OtherBodyIndex :type Integer))
  (Rendering|SetVisibility (Variables|Default|GetInteractionComunication) false false)
  (Utilities|Casting|CastToBP_TopDown_Char OtherActor)
  (Input|DisableInput (Game|GetPlayerController 0)))

(event Input|KeyboardEvents|E
  (params (Key :type Key%20Structure))
  (:Pressed
    (Development|PrintString "Aktywacja drzwi")
    (Transformation|SetActorLocation (Game|GetPlayerCharacter 0) (Variables|Default|GetNew%20Location) false false)))

(fn ConstructionScript)