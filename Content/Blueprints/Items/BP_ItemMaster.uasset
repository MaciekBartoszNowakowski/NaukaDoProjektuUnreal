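; BP_ItemMaster is a pickup item actor, named as the master item, that the top-down character collects with the E key.
; A sphere overlap with BP_TopDown_Char enables input on the item for player controller 0, and end overlap disables it.
; Pressing E casts the overlap's OtherActor to the character, passes ItemInfo to its PickUpItemEvent and destroys the item.
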(event OnComponentBeginOverlap(Sphere)
  (params (OverlappedComponent :type Primitive%20Component%20Object%20Reference) (OtherActor :type Actor%20Object%20Reference) (OtherComp :type Primitive%20Component%20Object%20Reference) (OtherBodyIndex :type Integer) (bFromSweep :type Boolean) (SweepResult :type Hit%20Result%20Structure%20%28by%20ref%29))
  (Utilities|Casting|CastToBP_TopDown_Char OtherActor)
  (Input|EnableInput (Game|GetPlayerController 0)))

(event OnComponentEndOverlap(Sphere)
  (params (OverlappedComponent :type Primitive%20Component%20Object%20Reference) (OtherActor :type Actor%20Object%20Reference) (OtherComp :type Primitive%20Component%20Object%20Reference) (OtherBodyIndex :type Integer))
  (Utilities|Casting|CastToBP_TopDown_Char OtherActor)
  (Input|DisableInput (Game|GetPlayerController 0)))

(event Input|KeyboardEvents|E
  (params (Key :type Key%20Structure :default "None"))
  (:Pressed
    (bind _asbp_top_down_char (Utilities|Casting|CastToBP_TopDown_Char (stale OnComponentBeginOverlap(Sphere) OtherActor)))
    (Default|PickUpItemEvent _asbp_top_down_char (Variables|Default|GetItemInfo))
    (Actor|DestroyActor)))

(fn ConstructionScript)