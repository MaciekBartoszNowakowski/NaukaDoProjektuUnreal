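; BP_Sheep is an NPC sheep that wanders randomly and flees when the player's top-down character gets close.
; BeginPlay caches the player, then starts a roaming loop of AIMoveTo calls to random reachable points and a recursive, delay-based proximity check using summed X/Y distance.
; RunAway moves directly away from the player, repeating while they stay near, otherwise resuming roaming.
; Both movement events continue only on move success, with no failure handling.
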(event Custom|Roam%20Around
  (AI|AIMoveTo self (.RandomLocation (AI|Navigation|GetRandomReachablePointinRadius (Transformation|GetActorLocation) 5e+02 0 0)) 0 1.2e+02 false
    (:OnSuccess
      (Utilities|FlowControl|Delay 1.2)
      (CallFunction|RoamAround))))

(event Custom|Run%20Away
  (bind _returnvalue (Transformation|GetActorLocation))
  (bind _returnvalue_2 (Transformation|GetActorLocation))
  (bind _charref (Variables|Default|GetCharRef))
  (bind _charref_2 (Variables|Default|GetCharRef))
  (bind _returnvalue_3 (Transformation|GetActorLocation _charref))
  (bind _returnvalue_4 (Transformation|GetActorLocation _charref_2))
  (bind _returnvalue_5 (Math|Rotator|FindLookatRotation _returnvalue_2 _returnvalue_3))
  (bind _returnvalue_6 (- _returnvalue _returnvalue_4))
  (bind _returnvalue_7 (Math|Vector|GetForwardVector _returnvalue_5))
  (bind _returnvalue_8 (* _returnvalue_7 "-500.000000,-500.000000,0.000000"))
  (bind _returnvalue_9 (+ _returnvalue_2 _returnvalue_8))
  (bind (_x _y) (Math|Vector|BreakVector _returnvalue_9))
  (AI|AIMoveTo self (Math|Vector|MakeVector _x _y (.Z (Math|Vector|BreakVector _returnvalue_2))) 0 2e+02 false
    (:OnSuccess
      (if (< (+ (Math|Float|Absolute(Float) (.x _returnvalue_6)) (Math|Float|Absolute(Float) (.y _returnvalue_6))) 2e+02)
        (CallFunction|RunAway)
        (else
          (CallFunction|RoamAround))))))

(event Custom|Running%20Check
  (bind _returnvalue (Transformation|GetActorLocation))
  (bind _charref (Variables|Default|GetCharRef))
  (bind _returnvalue_2 (Transformation|GetActorLocation _charref))
  (bind _returnvalue_3 (- _returnvalue _returnvalue_2))
  (if (< (+ (Math|Float|Absolute(Float) (.x _returnvalue_3)) (Math|Float|Absolute(Float) (.y _returnvalue_3))) 2e+02)
    (CallFunction|RunAway))
  (Utilities|FlowControl|Delay 0.1)
  (CallFunction|RunningCheck))

(event EventBeginPlay
  (bind _asbp_top_down_char (Utilities|Casting|CastToBP_TopDown_Char (Game|GetPlayerCharacter 0)))
  (Variables|Default|SetCharRef _asbp_top_down_char)
  (CallFunction|RoamAround)
  (CallFunction|RunningCheck))

(fn ConstructionScript)